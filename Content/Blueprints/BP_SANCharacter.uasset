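; BP_SANCharacter is a player character with axis-driven movement and mouse look.
; Forward and Right axes move it along the actor's own vectors, while MouseX and MouseY feed controller yaw and pitch.
; A ChangeLevel event teleports it vertically by a given Z offset without sweeping, keeping X and Y.
; GetCameraForward exposes the Camera component's forward vector.
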(event `self.ReceiveBeginPlay`)

(event `InputAxis|Forward`
  (params (AxisValue :type "Float (single-precision)"))
  (`self.AddMovementInput` (`self.GetActorForwardVector`) AxisValue))

(event `self.ReceiveActorBeginOverlap`
  (params (OtherActor :type "Actor Object Reference")))

(event `ChangeLevel`
  (params (LevelZ :type "Float (double-precision)"))
  (bind (_returnvalue_x _returnvalue_y _returnvalue_z) (`KismetMathLibrary.BreakVector` (`self.K2_GetActorLocation`)))
  (`self.K2_SetActorLocation` (`KismetMathLibrary.MakeVector` _returnvalue_x _returnvalue_y (+ _returnvalue_z LevelZ)) false true))

(event `InputAxis|Right`
  (params (AxisValue :type "Float (single-precision)"))
  (`self.AddMovementInput` (`self.GetActorRightVector`) AxisValue))

(event `self.ReceiveTick`
  (params (DeltaSeconds :type "Float (single-precision)")))

(event `InputAxis|MouseX`
  (params (AxisValue :type "Float (single-precision)"))
  (`self.AddControllerYawInput` AxisValue))

(event `InputAxis|MouseY`
  (params (AxisValue :type "Float (single-precision)"))
  (`self.AddControllerPitchInput` AxisValue))

(fn `GetCameraForward`
  (returns (CameraForward :type "Vector Structure"))
  (return (`SceneComponent.GetForwardVector` (`self.Camera`))))

(fn `UserConstructionScript`)