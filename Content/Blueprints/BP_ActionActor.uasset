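; BP_ActionActor is an actor that fires a one-time event when a character looks at it.
; ActivateLookAt and DeactivateLookAt set or clear the watched character.
; Tick compares the dot product of that camera's forward vector and its direction to the actor against Threshold.
; Exceeding it clears the character, calls OnLookingAtMe and sets Done to prevent retriggering.
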(event `self.ReceiveBeginPlay`)

(event `ActivateLookAt`
  (params (Character :type "/Game/Blueprints/BP_SANCharacter Object Reference"))
  (set `self.LookingCharacter` Character))

(event `DeactivateLookAt`
  (set `self.LookingCharacter` null))

(event `self.ReceiveActorBeginOverlap`
  (params (OtherActor :type "Actor Object Reference")))

(event `self.ReceiveTick`
  (params (DeltaSeconds :type "Float (single-precision)"))
  (bind _camera (`/Game/Blueprints/BP_SANCharacter.Camera` (`self.LookingCharacter`)))
  (if (not (`self.Done?`))
    (`/Engine/EditorBlueprintResources/StandardMacros.IsValid` (`self.LookingCharacter`)
      (:`Is Valid`
        (`|ExecutionSequence`
          (:`then_0`
            (set `self.FromCamera` (`SceneComponent.GetForwardVector` _camera))
            (set `self.ToCamera` (`KismetMathLibrary.Normal` (- (`self.K2_GetActorLocation`) (`SceneComponent.K2_GetComponentLocation` _camera)))))
          (:`then_1`
            (bind _output_get (set `self.Result` (`KismetMathLibrary.Dot_VectorVector` (`self.FromCamera`) (`self.ToCamera`))))
            (if (> _output_get (`self.Threshold`))
              (`self.DeactivateLookAt`)
              (`self.OnLookingAtMe`)
              (set `self.Done?` true))))))))

(fn `OnRep_Threshold`)

(fn `UserConstructionScript`)